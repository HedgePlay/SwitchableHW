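; BP_Light is a light actor that a linked Switcher turns on and off.
; On BeginPlay it applies LightColor to its PointLight and binds SwitchOff to the Switcher's OnPressed dispatcher.
; Despite its name, SwitchOff toggles the light's visibility and the IsOn flag on each press.
; IsSwitchOn exposes that flag as the current state.
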(event `self.ReceiveBeginPlay`
  (add `/Game/InterfaceLearning/Actors/BP_Switcher.OnPressed` (`self.Switcher`) (delegate `/Game/InterfaceLearning/Interfaces/BPI_Switchable.SwitchOff`))
  (`LightComponent.SetLightColor` (`self.PointLight`) (`self.LightColor`) true))

(event `/Game/InterfaceLearning/Interfaces/BPI_Switchable.SwitchOff`
  (bind _pointlight (`self.PointLight`))
  (if (`self.IsOn`)
    (`SceneComponent.SetVisibility` _pointlight false false)
    (set `self.IsOn` false)
    (else
      (`SceneComponent.SetVisibility` _pointlight true false)
      (set `self.IsOn` true))))

(fn `IsSwitchOn`
  (returns (IsOn :type Boolean))
  (return (`self.IsOn`)))

(fn `UserConstructionScript`)